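; Base weapon actor providing hitscan single and automatic fire with server-side ammo and damage.
; The client sphere-traces from the camera with random spread, re-traces from the muzzle to that point, then sends the result to the server.
; Auto fire loops through a gated delay; the server decrements ammo, applies damage, or stops the character firing at zero.
; Reload and fire FX functions are empty stubs.
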(event Custom|Server_ShootInfo
  (params (OutHit :type Hit%20Result%20Structure%20%28by%20ref%29) (Hit :type Boolean) (SeeProjectileSpawnLoc :type Vector) (NoSeeProjectileSpawnLoc :type Vector))
  (bind _bpmaincharacter (Variables|Default|GetBPMainCharacter))
  (Variables|Default|SetCurrentAmmoInclip (Math|Integer|Clamp(Integer) (- (Variables|Default|GetCurrentAmmoInclip) 1) 0 (Variables|Default|GetMaxAmmo)))
  (if (not (== (Variables|Default|GetCurrentAmmoInclip) 0))
    (Game|Damage|ApplyDamage (.HitActor (Collision|BreakHitResult OutHit)) (Variables|Default|GetBase%20Damage) (Game|GetInstigatorController) self)
    (else
      (Utilities|IsValid _bpmaincharacter
        (:Is%20Valid
          (Default|ServerStopWaponFire _bpmaincharacter))))))

(event Custom|Client_OffWeaponFire
  (Utilities|FlowControl|Sequence
    (:then_0
      (Utilities|AutoFireMode) ; enters at Close
    )))

(event Custom|Clinet_OnWeaponFire
  (switch Utilities|FlowControl|Switch|SwitchonE_FiringMode (Variables|Default|GetFiringMode)
    (:NewEnumerator0
      _)
    (:NewEnumerator1
      (Utilities|AutoFireMode
        (:Completed
          _))))
  (bind (_outhit _hit _seeprojectilespawnloc _noseeprojectilespawnloc) (CallFunction|ShpereTrace))
  (CallFunction|ServerShootInfo _outhit _hit _seeprojectilespawnloc _noseeprojectilespawnloc))

(event EventBeginPlay
  (Networking|SwitchHasAuthority
    (:Authority
      (Variables|Default|SetCurrentMaxAmmo (Variables|Default|GetMaxAmmo))
      (Variables|Default|SetCurrentAmmoInclip (Variables|Default|GetMaxAmmoClipSize)))))

(event Collision|EventActorBeginOverlap
  (params (OtherActor :type Actor%20Object%20Reference)))

(event EventTick
  (params (DeltaSeconds :type Float%20%28single-precision%29)))

(fn ConstructionScript)

(fn ShpereTrace
  (bind _returnvalue (Game|GetPlayerCameraManager 0))
  (bind _returnvalue_2 (Utilities|Name|MakeLiteralName "Muzzle"))
  (bind _returnvalue_3 (Math|Float|MakeLiteralFloat 2.0))
  (bind _returnvalue_4 (Components|GetOwner))
  (bind _sk_rifle_see (Variables|Default|GetSK_Rifle_See))
  (bind _returnvalue_5 (Camera|GetCameraLocation _returnvalue))
  (bind _returnvalue_6 (Transformation|GetSocketLocation _sk_rifle_see _returnvalue_2))
  (bind _array (Utilities|Array|MakeArray _returnvalue_4))
  (bind (_outhit _returnvalue_7) (Collision|SphereTraceByChannel _returnvalue_5 (+ (+ _returnvalue_5 (* (Math|Vector|GetForwardVector (Camera|GetCameraRotation _returnvalue)) 1e+04)) (* (Math|Random|RandomFloatinRange 0.0 3e+02) (Math|Random|RandomUnitVector))) _returnvalue_3 "TraceTypeQuery1" false _array "None"))
  (bind (_outhit_2 _returnvalue_8) (Collision|SphereTraceByChannel _returnvalue_6 (Math|Vector|SelectVector (.ImpactPoint (Collision|BreakHitResult _outhit)) (.TraceEnd (Collision|BreakHitResult _outhit)) _returnvalue_7) _returnvalue_3 "TraceTypeQuery1" false _array "ForDuration"))
  (return _outhit_2 _returnvalue_8 _returnvalue_6 (Transformation|GetSocketLocation (Variables|Default|GetSK_Rifle1_NoSee) _returnvalue_2)))

(fn ReloadAddAmoo)

(fn FireFx)